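; Activatable sliding double door that opens once when its Activate/Deactivate event fires.
; The event stores both cubes' relative locations, then passes through a DoOnce to play a timeline that offsets them in opposite directions along local X.
; The DoOnce is never reset and the timeline never reverses, so the door does not close, though later calls still overwrite the stored locations.
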(event `self.Activate/Deactivate`
  (bind (_relative_location_cube_x _relative_location_cube_y _relative_location_cube_z) (`KismetMathLibrary.BreakVector` (`self.Relative Location Cube`)))
  (bind (_relative_location_cube_1_x _relative_location_cube_1_y _relative_location_cube_1_z) (`KismetMathLibrary.BreakVector` (`self.Relative Location Cube 1`)))
  (set `self.Relative Location Cube 1` (`SceneComponent.RelativeLocation` (`self.Cube1`)))
  (set `self.Relative Location Cube` (`SceneComponent.RelativeLocation` (`self.Cube`)))
  (`/Engine/EditorBlueprintResources/StandardMacros.DoOnce` false
    (:`Completed`
      (bind (_direction _newtrack_0) (`Timeline|Timeline`)
        (:`Update`
          (`SceneComponent.K2_SetRelativeLocation` (`self.Cube`) (`KismetMathLibrary.MakeVector` (+ (* _newtrack_0 -1.0) _relative_location_cube_x) _relative_location_cube_y _relative_location_cube_z) false false)
          (`SceneComponent.K2_SetRelativeLocation` (`self.Cube1`) (`KismetMathLibrary.MakeVector` (+ _newtrack_0 _relative_location_cube_1_x) _relative_location_cube_1_y _relative_location_cube_1_z) false false))))))

(fn `UserConstructionScript`
  (`parent.UserConstructionScript`))